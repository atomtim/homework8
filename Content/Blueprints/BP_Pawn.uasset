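; Player pawn for a ball game that slides sideways and keeps a ball in play.
; The Moving Left axis applies fixed-step, swept world offsets along Y in either direction, based only on the input's sign.
; On BeginPlay it spawns a BP_Ball at its capsule's location, stores it and binds to its OnDead event, apparently to respawn a replacement through the SpawnBall event.
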(event Custom|Spawn%20Ball
  ;[0.4062 1 1] SPAWN BALL
  (CallFunction|SpawnBall))

(event EventBeginPlay
  ;[0.4062 1 1] SPAWN BALL
  (CallFunction|SpawnBall))

(event Input|AxisEvents|InputAxisMovingLeft
  (params (AxisValue :type Float%20%28single-precision%29))
  ;[0 1 0.1289] Player Control
  (if (> AxisValue 0.0)
    (Transformation|AddActorWorldOffset "0,-5.000000, 0" true)))

(event Input|AxisEvents|InputAxisMovingLeft
  (params (AxisValue :type Float%20%28single-precision%29))
  ;[0 1 0.1289] Player Control
  (if (< AxisValue 0.0)
    (Transformation|AddActorWorldOffset "0,5.000000, 0" true)))

(fn ConstructionScript)

(fn SpawnBall
  (bind _returnvalue (Game|SpawnActorfromClass "/Game/Blueprints/BP_Ball.BP_Ball_C" (Math|Conversions|ToTransform(Vector) (Transformation|GetWorldLocation (Variables|Default|GetCapsule))) "AlwaysSpawn" 0 0))
  (bind _output_get (Variables|Default|SetPlaying%20Ball _returnvalue))
  (EventDispatchers|BindEventtoOnDead _output_get (EventDispatchers|CreateEvent :!event Custom|Spawn%20Ball))
  (return 0))